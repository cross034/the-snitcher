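; AI controller for a chaser enemy that runs BT_Chaser and stores the ThirdPersonCharacter in the Blackboard as EnemyActor on possess.
; AI perception updates for actors tagged Player set HasPerceivedPlayer when sensed.
; Losing the stimulus starts a LineOfSightTimer delay before clearing the flag, and sensing again cancels it.
; A SensePlayer event sets the flag directly and cancels that timer.
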(event `self.ReceiveTick`
  (params (DeltaSeconds :type "Float (single-precision)")))

(event `self.ReceivePossess`
  (params (PossessedPawn :type "Pawn Object Reference"))
  (`self.RunBehaviorTree` "/Game/Blueprints/AI/BT_Chaser.BT_Chaser")
  (bind _returnvalue (`GameplayStatics.GetActorOfClass` "/Game/Blueprints/ThirdPersonCharacter.ThirdPersonCharacter_C"))
  (`BlackboardComponent.SetValueAsObject` (`self.Blackboard`) (`self.EnemyActor`) _returnvalue))

(event `self.AIPerception.OnTargetPerceptionUpdated`
  (params (Actor :type "Actor Object Reference") (Stimulus :type "AIStimulus Structure"))
  (if (`self.ActorHasTag` Actor "Player")
    (if (`.bSuccessfullySensed` (break `AIStimulus` Stimulus))
      (`KismetSystemLibrary.K2_ClearAndInvalidateTimerHandle` (`self.Enemy Timer`))
      (`BlackboardComponent.SetValueAsBool` (`self.Blackboard`) (`self.HasPerceivedPlayer`) true)
      (else
        (bind _returnvalue (`KismetSystemLibrary.K2_SetTimerDelegate` (delegate `Start Enemy Timer`) (`self.Line Of Sight Timer`)))
        (set `self.Enemy Timer` _returnvalue)))))

(event `Start Enemy Timer`
  (`BlackboardComponent.SetValueAsBool` (`self.Blackboard`) (`self.HasPerceivedPlayer`) false))

(event `Sense Player`
  (`BlackboardComponent.SetValueAsBool` (`self.Blackboard`) (`self.HasPerceivedPlayer`) true)
  (`KismetSystemLibrary.K2_ClearAndInvalidateTimerHandle` (`self.Enemy Timer`)))

(fn `UserConstructionScript`)