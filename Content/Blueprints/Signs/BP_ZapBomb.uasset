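; Zap bomb sign spell that homes in on a target enemy and detonates after a delay, using IgniBomb stats.
; Once cast, Tick sweeps the hit shape toward the target.
; Overlapping a non-ignored actor stops it; enemies also take initial damage and start the Burst timer.
; With VisualizeCast on, Burst spawns a radius visual, damages Enemy-tagged actors near the victim, then destroys itself; with it off, Burst does nothing.
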(event `Cast Attack`
  (params (Caster :type "Actor Object Reference (by ref)") (`Target Enemy` :type "Actor Object Reference (by ref)"))
  (bind _output_get (set `self.Caster` Caster))
  (set `self.Target Enemy` `Target Enemy`)
  (`KismetArrayLibrary.Array_Add` (`self.Actors to Ignore`) _output_get)
  (`SceneComponent.SetVisibility` (`self.Hit Detect Shape`) (`self.Visualize Cast`) false)
  (set `self.Is Casting` true))

(event `self.ReceiveTick`
  (params (DeltaSeconds :type "Float (single-precision)"))
  (bind _returnvalue (`KismetMathLibrary.FindLookAtRotation` (`SceneComponent.K2_GetComponentLocation` (`self.Hit Detect Shape`)) (`self.K2_GetActorLocation` (`self.Target Enemy`))))
  (set `self.Delta Seconds` DeltaSeconds)
  (if (`self.Is Casting`)
    (`SceneComponent.K2_SetWorldRotation` (`self.Hit Detect Shape`) _returnvalue false false)
    (`SceneComponent.K2_AddWorldOffset` (`self.Hit Detect Shape`) (* (`KismetMathLibrary.GetForwardVector` _returnvalue) (* (`self.Delta Seconds`) (`.IgniBombSpeed_33_42E1717D4E5B82829BA54CA352557298` (break `/Game/Blueprints/S_Stats` (`self.Stats`))))) true false)
    (else
      (`SceneComponent.SetVisibility` (`self.Hit Detect Shape`) false false))))

(event `self.Hit Detect Shape.OnComponentBeginOverlap`
  (params (OverlappedComponent :type "PrimitiveComponent Object Reference") (OtherActor :type "Actor Object Reference") (OtherComp :type "PrimitiveComponent Object Reference") (OtherBodyIndex :type Integer) (bFromSweep :type Boolean) (SweepResult :type "HitResult Structure (by ref)"))
  (bind (_ignidamage _ignibombinitdamage _ignibombblastdamage _ignibombspeed _ignibombdelay _ignibombradius) (break `/Game/Blueprints/S_Stats` (`self.Stats`)))
  (if (`self.Is Casting`)
    (if (`KismetArrayLibrary.Array_Contains` (`self.Actors to Ignore`) OtherActor)
      _
      (elif (`self.ActorHasTag` OtherActor "Enemy")
        (`KismetArrayLibrary.Array_AddUnique` (`self.Actors to Ignore`) OtherActor)
        (message `/Game/Blueprints/BPI_Enemy.Get Hit` OtherActor _ignibombinitdamage)
        (set `self.Is Casting` false)
        (set `self.Hit Enemy` OtherActor)
        (`KismetSystemLibrary.K2_SetTimerDelegate` (delegate `Burst`) _ignibombdelay)
        (else
          (set `self.Is Casting` false))))))

(event `Burst`
  (bind (_ignidamage _ignibombinitdamage _ignibombblastdamage _ignibombspeed _ignibombdelay _ignibombradius) (break `/Game/Blueprints/S_Stats` (`self.Stats`)))
  (if (`self.Visualize Cast`)
    (bind _returnvalue (`|SpawnActorFromClass` "/Game/Blueprints/Signs/BP_VisualizeBomb.BP_VisualizeBomb_C" (`KismetMathLibrary.MakeTransform` (`self.K2_GetActorLocation` (`self.Hit Enemy`)) (struct) (`KismetMathLibrary.Conv_DoubleToVector` (/ (`.IgniBombRadius_32_638845C84B7269567BABF294FB2AC01A` (break `/Game/Blueprints/S_Stats` (`self.Stats`))) 50.0))) "Undefined" "OverrideRootScale" null null))
    (`/Game/Blueprints/Signs/BP_VisualizeBomb.Destroy With Delay` _returnvalue 1.0)
    (bind _outactors (`GameplayStatics.GetAllActorsWithTag` "Enemy"))
    (for _array_element _outactors
      (if (<= (`self.GetDistanceTo` _array_element (`self.Hit Enemy`)) _ignibombradius)
        (message `/Game/Blueprints/BPI_Enemy.Get Hit` _array_element _ignibombblastdamage)))
    (`KismetSystemLibrary.Delay` 2.0)
    (`self.K2_DestroyActor`)))

(fn `UserConstructionScript`)