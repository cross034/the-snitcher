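; BP_GroundUp is a Yrden-style ground sign that creates a timed zone slowing actors inside it, ignoring the caster.
; While ShouldMoveCast is set, look input slides the zone relative to camera yaw; first movement reveals the blocker mesh and selects the moved-cast duration.
; Activation slows overlapping pawns and later entrants through message calls, using an ignore list against repeats.
; Leaving the active zone removes the debuff; a timer destroys the actor.
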(event `Initiate Cast`
  (params (Caster :type "Actor Object Reference (by ref)"))
  (bind _output_get (set `self.Caster` Caster))
  (`KismetArrayLibrary.Array_Add` (`self.Actors to Ignore`) _output_get)
  (`SceneComponent.SetVisibility` (`self.Hit Detect Shape`) (`self.Visualize Cast`) false)
  (bind _asthird_person_character (cast `/Game/Blueprints/ThirdPersonCharacter` (`self.Caster`)))
  (bind _output_get_2 (set `self.Player` _asthird_person_character))
  (set `self.Init Location` (`SceneComponent.K2_GetComponentLocation` (`Character.Mesh` _output_get_2)))
  (set `self.Is Casting` true))

(event `self.ReceiveTick`
  (params (DeltaSeconds :type "Float (single-precision)"))
  (bind _player (`self.Player`))
  (bind _movement_sensetivity (`self.Movement Sensetivity`))
  (bind (_returnvalue_roll _returnvalue_pitch _returnvalue_yaw) (`KismetMathLibrary.BreakRotator` (`Controller.GetControlRotation` (`GameplayStatics.GetPlayerController` 0))))
  (bind _returnvalue (`KismetMathLibrary.MakeRotator` 0.0 0.0 _returnvalue_yaw))
  (if (`self.Should Move Cast`)
    (bind _output_get (set `self.Delta Location` (+ (* (`KismetMathLibrary.GetForwardVector` _returnvalue) (* -1 (* (`/Game/Blueprints/ThirdPersonCharacter.Input Axis LookUp Value` _player) _movement_sensetivity))) (* (`KismetMathLibrary.GetRightVector` _returnvalue) (* _movement_sensetivity (`/Game/Blueprints/ThirdPersonCharacter.Input Axis Turn Value` _player))))))
    (`|ExecutionSequence`
      (:`then_0`
        (if (and (!= (`self.Delta Location`) (0.0 0.0 0.0)) (not (`self.Movement Detected`)))
          (set `self.Movement Detected` true)
          (`SceneComponent.SetVisibility` (`self.Projectile Blocker Mesh`) true false)))
      (:`then_1`
        (`SceneComponent.K2_AddWorldOffset` (`self.Hit Detect Shape`) _output_get false false)))))

(event `Activate Cast`
  (bind (_ignidamage _ignibombinitdamage _ignibombblastdamage _ignibombspeed _ignibombdelay _ignibombradius _yrdenspeeddebuff _yrdenduration _yrdenmovedduration) (break `/Game/Blueprints/S_Stats` (`self.Stats`)))
  (`PrimitiveComponent.SetMaterial` (`self.Hit Detect Shape`) 0 "/Game/Materials/MI_SlowActivated.MI_SlowActivated")
  (`KismetSystemLibrary.K2_SetTimerDelegate` (delegate `Deactivate`) (`KismetMathLibrary.SelectFloat` _yrdenmovedduration _yrdenduration (`self.Movement Detected`)))
  (set `self.Is Cast Active` true)
  (for _array_element (`PrimitiveComponent.GetOverlappingActors` (`self.Hit Detect Shape`) "/Script/Engine.Pawn")
    (if (`self.Is Cast Active`)
      (if (not (`KismetArrayLibrary.Array_Contains` (`self.Actors to Ignore`) _array_element))
        (`KismetArrayLibrary.Array_AddUnique` (`self.Actors to Ignore`) _array_element)
        (message `/Game/Blueprints/BPI_Enemy.Get Slow` _array_element (`.YrdenSpeedDebuff_10_952376CF464BBEEA331DCEA0D712BFC3` (break `/Game/Blueprints/S_Stats` (`self.Stats`))))))))

(event `Deactivate`
  (`self.K2_DestroyActor`))

(event `self.Hit Detect Shape.OnComponentBeginOverlap`
  (params (OverlappedComponent :type "PrimitiveComponent Object Reference") (OtherActor :type "Actor Object Reference") (OtherComp :type "PrimitiveComponent Object Reference") (OtherBodyIndex :type Integer) (bFromSweep :type Boolean) (SweepResult :type "HitResult Structure (by ref)"))
  (if (`self.Is Cast Active`)
    (if (not (`KismetArrayLibrary.Array_Contains` (`self.Actors to Ignore`) OtherActor))
      (`KismetArrayLibrary.Array_AddUnique` (`self.Actors to Ignore`) OtherActor)
      (message `/Game/Blueprints/BPI_Enemy.Get Slow` OtherActor (`.YrdenSpeedDebuff_10_952376CF464BBEEA331DCEA0D712BFC3` (break `/Game/Blueprints/S_Stats` (`self.Stats`)))))))

(event `self.Hit Detect Shape.OnComponentEndOverlap`
  (params (OverlappedComponent :type "PrimitiveComponent Object Reference") (OtherActor :type "Actor Object Reference") (OtherComp :type "PrimitiveComponent Object Reference") (OtherBodyIndex :type Integer))
  (if (`self.Is Cast Active`)
    (message `/Game/Blueprints/BPI_Enemy.Remove Speed Debuff` OtherActor)
    (if (!= (`self.Caster`) OtherActor)
      (`KismetArrayLibrary.Array_RemoveItem` (`self.Actors to Ignore`) OtherActor))))

(fn `UserConstructionScript`)