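; BP_Cast is a short-lived attack actor that deals damage along a stretching hit volume once CastAttack is called by a caster.
; Tick pushes HitDetectShape forward over Duration, scaling it toward full Length while interpolating its width.
; Overlaps during the cast send GetHitMessage with Damage once per actor, skipping the caster through an ignore list.
; Outside the cast window it hides and resets the shape, then destroys itself after a delay.
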(event `Cast Attack`
  (params (Caster :type "Actor Object Reference (by ref)"))
  (bind _output_get (set `self.Caster` Caster))
  (`KismetArrayLibrary.Array_Add` (`self.Actors to Ignore`) _output_get)
  (`SceneComponent.SetVisibility` (`self.Hit Detect Shape`) (`self.Visualize Cast`) false)
  (`SceneComponent.SetWorldScale3D` (`self.Hit Detect Shape`) (`KismetMathLibrary.MakeVector` (`self.Height`) (`self.Init Width`)))
  (set `self.Start Time` (`GameplayStatics.GetTimeSeconds`))
  (set `self.Is Casting` true))

(event `self.ReceiveTick`
  (params (DeltaSeconds :type "Float (single-precision)"))
  (bind _returnvalue (/ (- (`GameplayStatics.GetTimeSeconds`) (`self.Start Time`)) (`self.Duration`)))
  (bind _returnvalue_2 (* (`self.Length`) _returnvalue))
  (if (and (`self.Is Casting`) (<= (`GameplayStatics.GetTimeSeconds`) (+ (`self.Start Time`) (`self.Duration`))))
    (`SceneComponent.K2_SetRelativeLocation` (`self.Hit Detect Shape`) (`KismetMathLibrary.MakeVector` (* _returnvalue_2 300.0)) true false)
    (`SceneComponent.SetWorldScale3D` (`self.Hit Detect Shape`) (`KismetMathLibrary.MakeVector` (`self.Height`) (`KismetMathLibrary.Lerp` (`self.Init Width`) (`self.End Width`) _returnvalue) _returnvalue_2))
    (else
      (`SceneComponent.SetVisibility` (`self.Hit Detect Shape`) false false)
      (`SceneComponent.SetWorldScale3D` (`self.Hit Detect Shape`) (`KismetMathLibrary.MakeVector` (`self.Height`) (`self.Init Width`)))
      (set `self.Is Casting` false)
      (`KismetSystemLibrary.Delay` 2.0)
      (`self.K2_DestroyActor`))))

(event `self.Hit Detect Shape.OnComponentBeginOverlap`
  (params (OverlappedComponent :type "PrimitiveComponent Object Reference") (OtherActor :type "Actor Object Reference") (OtherComp :type "PrimitiveComponent Object Reference") (OtherBodyIndex :type Integer) (bFromSweep :type Boolean) (SweepResult :type "HitResult Structure (by ref)"))
  (if (`self.Is Casting`)
    (if (not (`KismetArrayLibrary.Array_Contains` (`self.Actors to Ignore`) OtherActor))
      (`KismetArrayLibrary.Array_AddUnique` (`self.Actors to Ignore`) OtherActor)
      (message `/Game/Blueprints/BPI_Enemy.Get Hit` OtherActor (`self.Damage`)))))

(fn `UserConstructionScript`)