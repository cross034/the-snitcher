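; Enemy AI character for melee combat that can lock onto targets and be locked by the player.
; It creates a screen-space state widget that follows a marker each tick, showing player lock state and cancelling that lock beyond a maximum distance.
; Its own lock scales attack lunge distance toward the target, capped before a boost multiplier.
; Getting hit alerts its chaser controller; death detaches the controller and notifies the player's lock system.
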(event `self.ReceiveTick`
  (params (DeltaSeconds :type "Float (single-precision)"))
  (bind _screenposition (`GameplayStatics.ProjectWorldToScreen` (`GameplayStatics.GetPlayerController` 0) (`SceneComponent.K2_GetComponentLocation` (`self.Marker Location`))))
  (`parent.ReceiveTick` DeltaSeconds)
  (`UserWidget.SetPositionInViewport` (`self.Enemy State UI`) (`KismetMathLibrary.MakeVector2D` (`KismetMathLibrary.BreakVector2D` _screenposition) (`.Y` (`KismetMathLibrary.BreakVector2D` _screenposition))) true)
  (bind _output_get (set `self.Distance To Player` (`KismetMathLibrary.Vector_Distance` (`self.K2_GetActorLocation`) (`self.K2_GetActorLocation` (`GameplayStatics.GetPlayerCharacter` 0)))))
  (if (and (> _output_get (`.LockMaxDistance_45_B14DF07E4E8EC789340369B10E678662` (break `/Game/Blueprints/S_Stats` (`self.Stats`)))) (`self.Is Locked By Player`))
    (`self.Cancel Lock` (cast `/Game/Blueprints/ThirdPersonCharacter` (`GameplayStatics.GetPlayerCharacter` 0) :!pure true))))

(event `Lock`
  (params (Enemy :type "Actor Object Reference"))
  (set `self.Locked Enemy` Enemy)
  (set `self.Is Enemy Locked` true)
  (`self.Enemy Lock Triggered` true Enemy))

(event `Check AI Lock Status Change` :!signature `self.Enemy Lock Triggered`
  (params (`Lock State` :type Boolean) (Enemy :type "Actor Object Reference"))
  (bind _output_get (set `self.Is Locked By Player` (and `Lock State` (== Enemy self))))
  (`/Game/UI/Enemy_State_UI.Change Lock UI State` (`self.Enemy State UI`) _output_get))

(event `Cancel Lock`
  (set `self.Locked Enemy` null)
  (set `self.Is Enemy Locked` false)
  (`self.Enemy Lock Triggered` false))

(event `self.ReceiveBeginPlay`
  (`parent.ReceiveBeginPlay`)
  (`/Game/Blueprints/BP_Sword.Ignore All Enemies` (`self.Sword`))
  (bind _returnvalue (`|CreateWidget` "/Game/UI/Enemy_State_UI.Enemy_State_UI_C"))
  (bind _output_get (set `self.Enemy State UI` _returnvalue))
  (set `/Game/UI/Enemy_State_UI.Owning Enemy` self _output_get)
  (`UserWidget.AddToViewport` (`self.Enemy State UI`) 0)
  (`|ExecutionSequence`
    (:`then_0`
      (add `self.Enemy Lock Triggered` (cast `/Game/Blueprints/ThirdPersonCharacter` (`GameplayStatics.GetPlayerCharacter` 0) :!pure true) (delegate `Check AI Lock Status Change`)))
    (:`then_1`
      (add `self.Starting Attack Montage` (delegate `Set Attack Boost`)))
    (:`then_2`
      (add `self.Character Died` (delegate `AI Character Died`)))))

(event `Set Attack Boost` :!signature `self.Starting Attack Montage`
  (params (Stage :type Integer))
  (if (`self.Is Enemy Locked`)
    (set `self.Attack Move Distance` (* (`KismetMathLibrary.FMin` (`KismetMathLibrary.Vector_Distance` (`self.K2_GetActorLocation`) (`self.K2_GetActorLocation` (`self.Locked Enemy`))) (`self.Max Attack Move Distance`)) 1.4))))

(event `AI Character Died`
  (`self.DetachFromControllerPendingDestroy`)
  (`self.Check Lock Status Of Dying Enemy` (cast `/Game/Blueprints/ThirdPersonCharacter` (`GameplayStatics.GetPlayerCharacter` 0) :!pure true) self)
  (`KismetSystemLibrary.Delay` 1.0)
  (set `self.Is Dead` true))

(event `/Game/Blueprints/BPI_Enemy.Get Hit`
  (params (Damage :type "Float (single-precision)"))
  (`parent.Get Hit` Damage)
  (bind _asaic_chaser (cast `/Game/Blueprints/AI/AIC_Chaser` (`self.GetController`)))
  (`/Game/Blueprints/AI/AIC_Chaser.Sense Player` _asaic_chaser))

(fn `Update Walk Speed`
  (params (`New Walk Speed` :type "Float (double-precision)"))
  (bind _output_get (set `self.Base Max Walk Speed` `New Walk Speed`))
  (set `CharacterMovementComponent.MaxWalkSpeed` (* _output_get (`self.Speed Multiplier`)) (`self.CharacterMovement`)))

(fn `UserConstructionScript`
  (`parent.UserConstructionScript`))