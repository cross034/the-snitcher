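; BP_Sword is a melee weapon actor that detects hit actors and toggles a trail effect.
; It caches world positions of six blade points, then sphere-traces from current to cached positions to cover the swept path, returning unique hit actors.
; Caching is separate from tracing and runs internally only at BeginPlay.
; Helper functions add one actor or all "Enemy"-tagged actors to the trace ignore list.
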(event `self.ReceiveTick`
  (params (DeltaSeconds :type "Float (single-precision)")))

(event `self.ReceiveBeginPlay`
  (set `self.Points Components` (`|MakeArray` (`self.Sword Point 1`) (`self.Sword Point 2`) (`self.Sword Point 3`) (`self.Sword Point 4`) (`self.Sword Point 5`) (`self.Sword Point 6`)))
  (`self.Cache Point Positions`)
  (`self.End Trail`))

(event `Start Trail`
  (`ActorComponent.Activate` (`self.Trail System`) false))

(event `End Trail`
  (`ActorComponent.Deactivate` (`self.Trail System`)))

(fn `Cache Point Positions`
  (for (_array_element _array_index) (`self.Points Components`)
    (`KismetArrayLibrary.Array_Set` (`self.Point Positions`) _array_index (`SceneComponent.K2_GetComponentLocation` _array_element) true)))

(fn `Ignore All Enemies`
  (bind _outactors (`GameplayStatics.GetAllActorsWithTag` "Enemy"))
  (for _array_element _outactors
    (`KismetArrayLibrary.Array_Add` (`self.Actors to Ignore`) _array_element)))

(fn `Set Actor To Ignore`
  (params (Actor :type "Actor Object Reference"))
  (`KismetArrayLibrary.Array_Add` (`self.Actors to Ignore`) Actor))

(fn `Trace For Enemies`
  (returns (`Hit Enemy` :type Boolean) (`Hit Enemy List` :type "Array of Actor Object Reference"))
  (bind _hit_actors (`self.Hit Actors`))
  (`KismetArrayLibrary.Array_Clear` (`self.Hit Actors`))
  (for (_array_element _array_index) (`self.Points Components`)
    (bind (_outhit _returnvalue) (`KismetSystemLibrary.SphereTraceSingleForObjects` (`SceneComponent.K2_GetComponentLocation` _array_element) (`|GetArrayItem` (`self.Point Positions`) _array_index) 5.0 (`self.Object Types`) false (`self.Actors to Ignore`) "None" true (struct :`R` 1.0 :`A` 1.0) (struct :`G` 1.0 :`A` 1.0) 0.1))
    (if _returnvalue
      (`KismetArrayLibrary.Array_AddUnique` (`self.Hit Actors`) (`.HitActor` (`GameplayStatics.BreakHitResult` _outhit)))))
  (return (> (`KismetArrayLibrary.Array_Length` _hit_actors) 0) _hit_actors))

(fn `UserConstructionScript`)